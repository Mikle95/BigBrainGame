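; Inventory component that stores item class and quantity stacks in a Columns × Rows slot array and shows them through a W_Inventory widget.
; AddItem fills the first empty or matching stack with space, recursing for any overflow, while RemoveItemAt reduces or clears a slot.
; Both refresh the affected slot widget.
; Selecting a tool slot spawns that BP_Base_Tool class at the player and equips it on PlayerRobot.
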(event `self.ReceiveBeginPlay`
  (`parent.ReceiveBeginPlay`)
  (`self.Resize`)
  (bind _asw_inventory (cast `/Game/Inventory/Widgets/W_Inventory` (`self.Widget`)))
  (`/Game/Inventory/Widgets/W_Inventory.SetParams` _asw_inventory (`self.Columns`) self)
  (`/Game/Inventory/Widgets/W_Inventory.PopulateSlotWidgets` _asw_inventory))

(event `ToggleInventoryGUI`
  (if (`self.GUIShown`)
    (`self.HideGUI`)
    (set `self.GUIShown` false)
    (else
      (`self.ShowGUI`)
      (set `self.GUIShown` true))))

(event `UpdateSlotAt`
  (params (Index :type Integer))
  (bind _asw_inventory (cast `/Game/Inventory/Widgets/W_Inventory` (`self.Widget_0`)))
  (`/Game/Inventory/Widgets/W_InventorySlot.UpdateSlot` (`|GetArrayItem` (`/Game/Inventory/Widgets/W_Inventory.SlotWidgets` _asw_inventory) Index)))

(event `SelectedTool`
  (params (InventoryIndex :type Integer))
  (bind _asbp_base_tool (castclass `/Game/Item/Blueprints/BP_Base_Tool` (`.Type_13_18AA60B24B1BF64830226BB28E2A0DAC` (break `/Game/Inventory/S_InventorySlot` (`|GetArrayItem` (`self.Slots`) InventoryIndex)))))
  (bind _tool (`self.SpawnToolFromInventory` _asbp_base_tool))
  (bind _asplayer_robot (cast `/Game/FirstPersonBP/Blueprints/PlayerRobot` (`GameplayStatics.GetPlayerCharacter` 0)))
  (`/Game/FirstPersonBP/Blueprints/PlayerRobot.Equip` _asplayer_robot _tool InventoryIndex))

(fn `AddItem`
  (params (Type :type "/Game/Item/Blueprints/BP_Base_Item Class Reference") (Amount :type Integer))
  (returns (Success :type Boolean) (Rest :type Integer))
  (locals (LeftToAdd :type Integer))
  (bind _slots (`self.Slots`))
  (bind _output_get (set `local.LeftToAdd` Amount))
  (bind (_index _found _freespace) (`self.FindFreeStack` Type))
  (if _found
    (bind _output_get_2 (set `local.LeftToAdd` (- (`local.LeftToAdd`) _freespace)))
    (`KismetArrayLibrary.Array_Set` _slots _index (make `/Game/Inventory/S_InventorySlot` (`KismetMathLibrary.Max` (+ (`.Quantity_3_5CE892F446C1A1E2EF5DD7B840D2CCA5` (break `/Game/Inventory/S_InventorySlot` (`|GetArrayItem` _slots _index))) (`local.Amount`)) (`.StackLimit_10_9D37F9174AF8BA7FF84AA7B3AC5C358E` (break `/Game/Item/S_ItemInfo` (defaults `Object` Type)))) Type))
    (`self.UpdateSlotAt` _index)
    (if (> _output_get_2 0)
      (bind (_success _rest) (`self.AddItem` Type _output_get_2)) ; If some items were not added, recursively add them
      (return true _rest)
      (else
        (return true 0)))
    (else
      (return false _output_get))))

(fn `FindFreeStack`
  (params (Type :type "/Game/Item/Blueprints/BP_Base_Item Class Reference"))
  (returns (Index :type Integer) (Found :type Boolean) (FreeSpace :type Integer))
  (bind (_name _description _icon _stacklimit) (break `/Game/Item/S_ItemInfo` (defaults `Object` Type)))
  (for (_array_element _array_index) (`self.Slots`)
    (bind (_quantity _type) (break `/Game/Inventory/S_InventorySlot` _array_element))
    (if (or (not (`KismetSystemLibrary.IsValidClass` _type)) (== _type Type))
      (if (< _quantity _stacklimit)
        (return _array_index true (- _stacklimit _quantity)))))
  (return 0 false 0))

(fn `GetItemInfoAt`
  (params (Index :type Integer))
  (returns (Empty :type Boolean) (Info :type "/Game/Item/S_ItemInfo Structure") (Number :type Integer))
  (bind (_quantity _type) (break `/Game/Inventory/S_InventorySlot` (`|GetArrayItem` (`self.Slots`) Index)))
  (if (`KismetSystemLibrary.IsValidClass` _type)
    (return false (defaults `Object` _type) _quantity)
    (else
      (return true (struct) 0))))

(fn `IsSlotEmpty`
  (params (Index :type Integer))
  (returns (Empty :type Boolean))
  (return (not (`KismetSystemLibrary.IsValidClass` (`.Type_13_18AA60B24B1BF64830226BB28E2A0DAC` (break `/Game/Inventory/S_InventorySlot` (`|GetArrayItem` (`self.Slots`) Index)))))))

(fn `RemoveItemAt`
  (params (Index :type Integer) (Amount :type Integer))
  (returns (Success :type Boolean))
  (bind _slots (`self.Slots`))
  (bind (_quantity _type) (break `/Game/Inventory/S_InventorySlot` (`|GetArrayItem` (`self.Slots`) Index)))
  (bind _returnvalue (- _quantity Amount))
  (if (`KismetSystemLibrary.IsValidClass` _type)
    (if (> _quantity 0)
      (if (> _returnvalue 0)
        (`KismetArrayLibrary.Array_Set` _slots Index (make `/Game/Inventory/S_InventorySlot` _returnvalue _type))
        (else
          (`KismetArrayLibrary.Array_Set` _slots Index)))
      (`self.UpdateSlotAt` Index)
      (return true)
      (else
        _)))
  (return false))

(fn `Resize`
  (`KismetArrayLibrary.Array_Resize` (`self.Slots`) (* (`self.Columns`) (`self.Rows`))))

(fn `SpawnToolFromInventory`
  (params (`Tool Type` :type "/Game/Item/Blueprints/BP_Base_Tool Class Reference"))
  (returns (Tool :type "/Game/Item/Blueprints/BP_Base_Tool Object Reference"))
  (bind _returnvalue (`|SpawnActorFromClass` `Tool Type` (`KismetMathLibrary.MakeTransform` (`Actor.K2_GetActorLocation` (`GameplayStatics.GetPlayerCharacter` 0))) "Undefined" "OverrideRootScale" null null true false null))
  (`Actor.K2_SetActorRelativeTransform` _returnvalue (`/Game/Item/Blueprints/BP_Base_Tool.RelativeTransform` _returnvalue) false false)
  (return _returnvalue))