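; Inventory Blueprint that stores item stacks as type and quantity in a Slots array, sized by Resize to Columns × Rows.
; Item info and stack limits come from each item class's defaults.
; AddItem uses FindFreeStack to pick the first empty or non-full matching slot, recursing on overflow, though it sets quantity with Max rather than clamping to the limit.
; ToggleGUI is a TODO that only flips VisibleGUI.
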(fn `AddItem`
  (params (Type :type "/Game/Item/Blueprints/BP_Base_Item Class Reference") (Amount :type Integer))
  (returns (Success :type Boolean) (Rest :type Integer))
  (locals (LeftToAdd :type Integer))
  (bind (_index _found _freespace) (`self.FindFreeStack` Type))
  (bind _slots (`self.Slots`))
  (bind _output_get (set `local.LeftToAdd` Amount))
  (if _found
    (bind _output_get_2 (set `local.LeftToAdd` (- (`local.LeftToAdd`) _freespace)))
    (`KismetArrayLibrary.Array_Set` _slots _index (make `/Game/Inventory/S_InventorySlot` (`KismetMathLibrary.Max` (+ (`.Quantity_3_5CE892F446C1A1E2EF5DD7B840D2CCA5` (break `/Game/Inventory/S_InventorySlot` (`|GetArrayItem` _slots _index))) (`local.Amount`)) (`.StackLimit_10_9D37F9174AF8BA7FF84AA7B3AC5C358E` (break `/Game/Item/ItemInfo` (defaults `Object` Type)))) Type))
    (if (> _output_get_2 0)
      (bind (_success _rest) (`self.AddItem` Type _output_get_2)) ; If some items were not added, recursively add them
      (return true _rest)
      (else
        (return true 0)))
    (else
      (return false _output_get))))

(fn `FindFreeStack`
  (params (Type :type "/Game/Item/Blueprints/BP_Base_Item Class Reference"))
  (returns (Index :type Integer) (Found :type Boolean) (FreeSpace :type Integer))
  (bind (_name _description _icon _stacklimit) (break `/Game/Item/ItemInfo` (defaults `Object` Type)))
  (for (_array_element _array_index) (`self.Slots`)
    (bind (_quantity _type) (break `/Game/Inventory/S_InventorySlot` _array_element))
    (if (or (not (`KismetSystemLibrary.IsValidClass` _type)) (== _type Type))
      (if (< _quantity _stacklimit)
        (return _array_index true (- _stacklimit _quantity)))))
  (return 0 false 0))

(fn `GetItemInfoAt`
  (params (Index :type Integer))
  (returns (Empty :type Boolean) (Info :type "/Game/Item/ItemInfo Structure") (Number :type Integer))
  (bind (_quantity _type) (break `/Game/Inventory/S_InventorySlot` (`|GetArrayItem` (`self.Slots`) Index)))
  (if (`KismetSystemLibrary.IsValidClass` _type)
    (return false (defaults `Object` _type) _quantity)
    (else
      (return true (struct) 0))))

(fn `IsSlotEmpty`
  (params (Index :type Integer))
  (returns (Empty :type Boolean))
  (return (not (`KismetSystemLibrary.IsValidClass` (`.Type_13_18AA60B24B1BF64830226BB28E2A0DAC` (break `/Game/Inventory/S_InventorySlot` (`|GetArrayItem` (`self.Slots`) Index)))))))

(fn `Resize`
  (`KismetArrayLibrary.Array_Resize` (`self.Slots`) (* (`self.Columns`) (`self.Rows`))))

(fn `ToggleGUI`
  (set `self.VisibleGUI` (not (`self.VisibleGUI`))) ; TODO
)

(fn `UserConstructionScript`)