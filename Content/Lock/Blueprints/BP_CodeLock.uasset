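; BP_CodeLock is a keypad code lock whose panel widget toggles when its parent is activated, tinting the RobotHUD background while shown.
; It creates CodeLock_Widget at BeginPlay, passing itself as CodePanel, and CipherEntered appends each input and updates the display.
; At the correct code's length, it compares and clears the entry; a match sets Open, hides the panel and blocks reopening.
; The door-opening signal remains a TODO.
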(event `self.ReceiveBeginPlay`
  (bind _returnvalue (`|CreateWidget` "/Game/Lock/Widgets/CodeLock_Widget.CodeLock_Widget_C" (`GameplayStatics.GetPlayerController` 0) self))
  (set `self.Widget` _returnvalue))

(event `ToggleGUI`
  (if (`KismetMathLibrary.BooleanNOR` (`self.Open`) (`self.GUIShown`))
    (`self.ShowGUI`)
    (set `self.GUIShown` true)
    (else
      (`self.HideGUI`)
      (set `self.GUIShown` false))))

(event `ParentActivated`
  (`self.ToggleGUI`))

(event `CipherEntered`
  (params (Cipher :type Integer))
  (bind _output_get (set `self.CurrentCode` (`KismetStringLibrary.Concat_StrStr` (`self.CurrentCode`) (`KismetStringLibrary.Conv_IntToString` Cipher))))
  (`/Game/Lock/Widgets/CodeLock_Widget.UpdateDisplay` (`self.Widget`) (`KismetTextLibrary.Conv_StringToText` _output_get))
  (if (>= (`KismetStringLibrary.Len` _output_get) (`KismetStringLibrary.Len` (`self.CorrectCode`)))
    (if (`KismetStringLibrary.EqualEqual_StrStr` (`self.CorrectCode`) (`self.CurrentCode`))
      (set `self.Open` true) ; TODO: send signal to open door
      (`self.HideGUI`))
    (set `self.CurrentCode` "")))

(fn `HideGUI`
  (bind _asrobot_hud (cast `/Game/FirstPersonBP/Blueprints/RobotHUD` (`PlayerController.GetHUD` (`GameplayStatics.GetPlayerController` 0))))
  (`/Game/FirstPersonBP/Blueprints/RobotHUD.UntintBackground` _asrobot_hud)
  (`Widget.RemoveFromParent` (`self.Widget`)))

(fn `ShowGUI`
  (bind _asrobot_hud (cast `/Game/FirstPersonBP/Blueprints/RobotHUD` (`PlayerController.GetHUD` (`GameplayStatics.GetPlayerController` 0))))
  (`/Game/FirstPersonBP/Blueprints/RobotHUD.TintBackground` _asrobot_hud)
  (`UserWidget.AddToViewport` (`self.Widget`) 0))