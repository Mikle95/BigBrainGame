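; InformationCarrier is a base Blueprint for in-game objects that present information to the player in an on-screen widget.
; It creates a widget of a configurable WidgetType at BeginPlay, and Activate toggles it on and off.
; Showing adds the widget to the viewport and tints the RobotHUD background, while hiding removes both and tracks the state in WidgetShown.
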(event `self.ReceiveBeginPlay`
  (bind _returnvalue (`|CreateWidget` (`self.WidgetType`)))
  (set `self.Widget` _returnvalue))

(event `/Game/FirstPersonBP/Blueprints/BPI_Activateble.Activate`
  (`self.ToggleGUI`))

(fn `HideWidget`
  (bind _asrobot_hud (cast `/Game/FirstPersonBP/Blueprints/RobotHUD` (`PlayerController.GetHUD` (`GameplayStatics.GetPlayerController` 0))))
  (`/Game/FirstPersonBP/Blueprints/RobotHUD.UntintBackground` _asrobot_hud)
  (`Widget.RemoveFromParent` (`self.Widget`))
  (set `self.WidgetShown` false))

(fn `ShowWidget`
  (bind _asrobot_hud (cast `/Game/FirstPersonBP/Blueprints/RobotHUD` (`PlayerController.GetHUD` (`GameplayStatics.GetPlayerController` 0))))
  (`/Game/FirstPersonBP/Blueprints/RobotHUD.TintBackground` _asrobot_hud)
  (`UserWidget.AddToViewport` (`self.Widget`) 0)
  (set `self.WidgetShown` true))

(fn `ToggleGUI`
  (if (`self.WidgetShown`)
    (`self.HideWidget`)
    (else
      (`self.ShowWidget`))))

(fn `UserConstructionScript`)