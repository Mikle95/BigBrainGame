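; BP_Base_Tool is a base item Blueprint for tools, with primary and secondary use actions.
; On BeginPlay, if Visible is set, it adds a skeletal mesh component with ToolSkeletalMesh so the tool shows on the ground.
; UsedPrimary and UsedSecondary events forward to PrimaryAction and SecondaryAction, which are empty here.
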(event `self.ReceiveBeginPlay`
  (if (`self.Visible`)
    (bind _returnvalue (`AddComponent|NODE_AddSkeletalMeshComponent-0`))
    (`SkinnedMeshComponent.SetSkinnedAssetAndUpdate` _returnvalue (`self.ToolSkeletalMesh`) true)))

(event `UsedPrimary`
  (`self.PrimaryAction`))

(event `UsedSecondary`
  (`self.SecondaryAction`))

(fn `PrimaryAction`)

(fn `SecondaryAction`)

(fn `UserConstructionScript`
  (`parent.UserConstructionScript`))