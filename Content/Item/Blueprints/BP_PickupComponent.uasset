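; BP_PickupComponent handles item pickups, moving a picked-up item into the inventory of a PlayerRobot.
; Its PickedUp event casts the other actor to PlayerRobot and, if the inventory is valid, adds the amount using the item actor's class as the type.
; On success, any leftover is written back to the item's Amount; otherwise the item actor is destroyed.
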(event `PickedUp`
  (params (OtherActor :type "Actor Object Reference") (ItemActor :type "/Game/Item/Blueprints/BP_Base_Item Object Reference") (Amount :type Integer))
  (bind _asplayer_robot (cast `/Game/FirstPersonBP/Blueprints/PlayerRobot` OtherActor))
  (bind _inventory (`/Game/FirstPersonBP/Blueprints/PlayerRobot.Inventory` _asplayer_robot))
  (if (`KismetSystemLibrary.IsValid` _inventory)
    (bind (_success _rest) (`/Game/Inventory/BP_Inventory.AddItem` _inventory (`GameplayStatics.GetObjectClass` ItemActor) Amount))
    (if _success
      (if (> _rest 0)
        (set `/Game/Item/Blueprints/BP_Base_Item.Amount` _rest ItemActor)
        (else
          (`Actor.K2_DestroyActor` ItemActor))))))