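; BP_Gun is a gun item that fires a first-person projectile through its PrimaryAction function.
; PrimaryAction plays the fire montage on the holder's skeletal mesh, then spawns the projectile at a camera-rotated offset, aimed along the camera.
; The spawn adjusts for collisions or is skipped if still blocked, and a firing sound plays at the gun's location.
; BeginPlay is disabled, and a leftover branch into the spawn is unreachable.
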(fn `PrimaryAction`
  (bind _firstpersoncamera (`self.FirstPersonCamera`))
  (bind _returnvalue (`SceneComponent.K2_GetComponentRotation` _firstpersoncamera))
  (`AnimInstance.Montage_Play` (`SkeletalMeshComponent.GetAnimInstance` (`self.HolderSkeletalMesh`)) "/Game/FirstPerson/Animations/FirstPersonFire_Montage.FirstPersonFire_Montage" 1.0 "MontageLength" 0.0 true)
  (`|SpawnActorFromClass` "/Game/FirstPersonBP/Blueprints/FirstPersonProjectile.FirstPersonProjectile_C" (`KismetMathLibrary.MakeTransform` (+ (`SceneComponent.K2_GetComponentLocation` _firstpersoncamera) (`KismetMathLibrary.GreaterGreater_VectorRotator` (`self.GunOffset`) _returnvalue)) _returnvalue) "AdjustIfPossibleButDontSpawnIfColliding" "OverrideRootScale" null null) ; Spawn projectile
  (`GameplayStatics.PlaySoundAtLocation` "/Game/FirstPerson/Audio/FirstPersonTemplateWeaponFire02.FirstPersonTemplateWeaponFire02" (`self.K2_GetActorLocation`) (struct) 1.0 1.0 0.0 null null null) ; Play firing sound
)

(fn `UserConstructionScript`
  (`parent.UserConstructionScript`))