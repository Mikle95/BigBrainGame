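; BP_ButtonWindow is a level element window that a linked button opens and closes.
; On BeginPlay it stores its starting location and registers itself as the Button's target Actor.
; Each Activate call flips a timeline between play and reverse.
; The timeline's DoorLoc value slides the window backward along its forward vector while shrinking its X scale, so it retracts as it moves.
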(event `self.ReceiveBeginPlay`
  (set `self.Pos` (`self.K2_GetActorLocation`))
  (set `/Game/LevelElements/BP_Button.Actor` self (`self.Button`)))

(event `/Game/FirstPersonBP/Blueprints/BPI_Activateble.Activate`
  (`/Engine/EditorBlueprintResources/StandardMacros.FlipFlop`
    (:`A`
      (bind (_direction _doorloc) (`Timeline|Timeline_0` :!label _label)
        (:`Update`
          (`self.K2_SetActorLocation` (+ (* (`self.GetActorForwardVector`) (* -1000 _doorloc)) (`self.Pos`)))
          (`self.SetActorScale3D` (`KismetMathLibrary.MakeVector` (* (`KismetMathLibrary.Abs` (- _doorloc 1.0)) 14.0) 4.0 0.25)))))
    (:`B`
      (goto _label :!via `Reverse`))))

(fn `UserConstructionScript`)