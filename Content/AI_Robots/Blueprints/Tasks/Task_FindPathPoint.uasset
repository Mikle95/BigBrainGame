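; Behavior tree task that picks the next patrol point for an enemy robot.
; It reads the robot's PatrolPath, offsets the point at the blackboard index by the path actor's location, and writes it to a blackboard vector.
; The index then advances with modulo wrapping to loop the path.
; The task finishes only on success; a failed cast or missing path never calls FinishExecute.
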(event `self.ReceiveExecuteAI`
  (params (OwnerController :type "AIController Object Reference") (ControlledPawn :type "Pawn Object Reference"))
  (bind _index (`self.Index`))
  (bind _returnvalue (`BTFunctionLibrary.GetBlackboardValueAsInt` _index))
  (bind _asbp_enemy_robot (cast `/Game/AI_Robots/Blueprints/BP_EnemyRobot` ControlledPawn))
  (bind _patrolpath (`/Game/AI_Robots/Blueprints/BP_EnemyRobot.PatrolPath` _asbp_enemy_robot)
    (:`then`
      (bind _pathpoints (`/Game/AI_Robots/Blueprints/BP_PatrolPath.PathPoints` _patrolpath))
      (`BTFunctionLibrary.SetBlackboardValueAsVector` (`self.Vector`) (+ (`Actor.K2_GetActorLocation` _patrolpath) (`|GetArrayItem` _pathpoints _returnvalue)))
      (`BTFunctionLibrary.SetBlackboardValueAsInt` _index (mod (+ 1 _returnvalue) (`KismetArrayLibrary.Array_Length` _pathpoints)))
      (`self.FinishExecute` true))
    (:`else`)))