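; Behavior tree task that lets an enemy robot deal an attack to the player robot.
; It checks the robot's Sphere for an overlapping PlayerRobot and calls AttackOnPlayer on the first one, passing the enemy's Attack value and itself as aggressor.
; The task succeeds after the hit and fails when no player is in the sphere.
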(event `self.ReceiveExecuteAI`
  (params (OwnerController :type "AIController Object Reference") (ControlledPawn :type "Pawn Object Reference"))
  (bind _asbp_enemy_robot (cast `/Game/AI_Robots/Blueprints/BP_EnemyRobot` ControlledPawn))
  (bind _overlappingactors (`PrimitiveComponent.GetOverlappingActors` (`/Game/AI_Robots/Blueprints/BP_EnemyRobot.Sphere` _asbp_enemy_robot) "/Game/FirstPersonBP/Blueprints/PlayerRobot.PlayerRobot_C"))
  (if (`KismetArrayLibrary.Array_IsValidIndex` _overlappingactors)
    (bind _asplayer_robot (cast `/Game/FirstPersonBP/Blueprints/PlayerRobot` (`|GetArrayItem` _overlappingactors)))
    (`/Game/FirstPersonBP/Blueprints/PlayerRobot.AttackOnPlayer` _asplayer_robot (`/Game/AI_Robots/Blueprints/BP_EnemyRobot.Attack` _asbp_enemy_robot) _asbp_enemy_robot)
    (`self.FinishExecute` true)
    (else
      (`self.FinishExecute` false))))