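; BP_CommunicationStation is a breakable AI relay that shares player-spotted alerts among guards registered with it.
; A spotted event raises the alert, then Tick keeps it while any connected guard reports the player visible.
; Changes in that state are pushed to every guard through SetAttackMode.
; Activate breaks the station and hides its mesh, blocking new alerts and making the visibility check return false.
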(event `self.ReceiveTick`
  (params (DeltaSeconds :type "Float (single-precision)"))
  ;[1 1 1] Communication
  (if (`self.PlayerSpotted`)
    (bind _result (`self.isPlayerVisible`))
    (bind _output_get (set `self.PlayerSpotted` _result))
    (if (!= _output_get (`self.AttackMode`))
      (set `self.AttackMode` _output_get)
      (for _array_element (`self.ConnectedGuards`)
        (`/Game/AI_Robots/Blueprints/AI/AI_Enemy_Controller.Set Attack Mode` _array_element (`self.PlayerSpotted`))))))

(event `player spotted`
  ;[1 1 1] Communication
  (set `self.PlayerSpotted` (not (`self.isBroken`))))

(event `/Game/FirstPersonBP/Blueprints/BPI_Activateble.Activate`
  ;[1 1 1] Breaking
  (set `self.isBroken` true)
  (`SceneComponent.SetVisibility` (`self.StaticMesh1`) false false))

(fn `isPlayerVisible`
  (returns (result :type Boolean))
  (locals (out :type Boolean))
  (if (`self.isBroken`)
    (return false)
    (else
      (for _array_element (`self.ConnectedGuards`)
        (bind _newparam (`/Game/AI_Robots/Blueprints/AI/AI_Enemy_Controller.GetPlayerVisibility` _array_element))
        (set `local.out` (or _newparam (`local.out`))))
      (return (`local.out`)))))

(fn `register`
  (params (Controller :type "/Game/AI_Robots/Blueprints/AI/AI_Enemy_Controller Object Reference"))
  (`/Engine/EditorBlueprintResources/StandardMacros.IsValid` Controller
    (:`Is Valid`
      (`KismetArrayLibrary.Array_Add` (`self.ConnectedGuards`) Controller))))

(fn `UserConstructionScript`)