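; AI controller for enemy robots that tracks whether the player robot is perceived.
; On BeginPlay it runs the BehaviorTree stored on its controlled BP_EnemyRobot pawn.
; AIPerception target updates for PlayerRobot actors write the sensed state to the CanSeePlayer blackboard key.
; GetPlayerVisibility reads that key back.
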(event `self.AIPerception.OnTargetPerceptionUpdated`
  (params (Actor :type "Actor Object Reference") (Stimulus :type "AIStimulus Structure"))
  (cast `/Game/FirstPersonBP/Blueprints/PlayerRobot` Actor)
  (`BlackboardComponent.SetValueAsBool` (`AIBlueprintHelperLibrary.GetBlackboard` null) "CanSeePlayer" (`.bSuccessfullySensed` (break `AIStimulus` Stimulus))))

(event `self.ReceiveBeginPlay`
  (bind _asbp_enemy_robot (cast `/Game/AI_Robots/Blueprints/BP_EnemyRobot` (`self.K2_GetPawn`)))
  (`self.RunBehaviorTree` (`/Game/AI_Robots/Blueprints/BP_EnemyRobot.BehaviorTree` _asbp_enemy_robot)))

(fn `GetPlayerVisibility`
  (returns (NewParam :type Boolean))
  (return (`BlackboardComponent.GetValueAsBool` (`AIBlueprintHelperLibrary.GetBlackboard` null) "CanSeePlayer")))

(fn `UserConstructionScript`)