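; Enemy robot Blueprint that tracks health, can be hacked by the player and collapses into a ragdoll at zero health.
; BeginPlay creates an HP/energy state with health only, which ChangeHealth modifies.
; Activate sets IsHacked when the player has a screwdriver equipped, true only if the blackboard's CanSeePlayer is false.
; CheckHealth, on depletion, unpossesses the controller once and enables mesh ragdoll physics.
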(event `/Game/FirstPersonBP/Blueprints/BPI_Activateble.Activate`
  (bind _asplayer_robot (cast `/Game/FirstPersonBP/Blueprints/PlayerRobot` (`GameplayStatics.GetPlayerPawn` 0)))
  (if (`KismetMathLibrary.ClassIsChildOf` (`GameplayStatics.GetObjectClass` (`/Game/FirstPersonBP/Blueprints/PlayerRobot.EquipedTool` _asplayer_robot)) "/Game/Item/Blueprints/BP_Screwdriver.BP_Screwdriver_C")
    (set `self.isHacked` (not (`BlackboardComponent.GetValueAsBool` (`AIBlueprintHelperLibrary.GetBlackboard` null) "CanSeePlayer")))))

(event `self.ReceiveBeginPlay`
  (bind _returnvalue (`AddComponent|NODE_AddHP_Energy_State-0` :`MaxHealth` (`self.Max Health`) :`Holder` self))
  (set `self.Hp_Energy` _returnvalue))

(event `/Game/Common/I_Has_HP_Energy.ChangeHealth`
  (params (value :type "Float (single-precision)"))
  (`/Game/Common/HP_Energy_State.ChangedHealth` (`self.Hp_Energy`) value false))

(event `/Game/Common/I_Has_HP_Energy.CheckHealth`
  (bind _mesh (`self.Mesh`))
  (bind _empty (`/Game/Common/HP_Energy_State.NoHealth` (`self.Hp_Energy`)))
  (if _empty
    (`/Engine/EditorBlueprintResources/StandardMacros.DoOnce` false
      (:`Completed`
        (`Controller.UnPossess` (`self.GetController`))
        (`PrimitiveComponent.SetCollisionProfileName` _mesh "Ragdoll" true)
        (`PrimitiveComponent.SetSimulatePhysics` _mesh true)))))

(fn `UserConstructionScript`)