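; BP_AutomaticDoor is an automatic door that opens when a FirstPersonCharacter is inside its Box and closes when none remains.
; Actor overlap events query the Box, and opening also requires IsActive, while closing does not.
; OpenDoor and CloseDoor set IsOpen, then both call MoveEvent, which is empty here, so this Blueprint defines no movement itself.
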(event `self.ReceiveActorBeginOverlap`
  (params (OtherActor :type "Actor Object Reference"))
  (if (and (`KismetArrayLibrary.Array_IsValidIndex` (`PrimitiveComponent.GetOverlappingActors` (`self.Box`) "/Game/FirstPersonBP/Blueprints/FirstPersonCharacter.FirstPersonCharacter_C")) (`self.isActive`))
    (`self.OpenDoor`)))

(event `self.ReceiveActorEndOverlap`
  (params (OtherActor :type "Actor Object Reference"))
  (if (not (`KismetArrayLibrary.Array_IsValidIndex` (`PrimitiveComponent.GetOverlappingActors` (`self.Box`) "/Game/FirstPersonBP/Blueprints/FirstPersonCharacter.FirstPersonCharacter_C")))
    (`self.CloseDoor`)))

(event `OpenDoor`
  (set `self.isOpen` true)
  (`self.MoveEvent` :!label _label))

(event `CloseDoor`
  (set `self.isOpen` false)
  (goto _label))

(event `MoveEvent`)

(fn `UserConstructionScript`)