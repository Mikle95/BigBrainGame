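; BP_HorizontalDoor is a two-panel door that animates between open and closed.
; MoveEvent plays or reverses the OpenClose timeline based on IsOpen, which is not set in this graph.
; The timeline value drives the pitch of Door1 and Door2, mounted at opposite yaws.
; Both panels also shrink uniformly from Door1's scale cached at BeginPlay as that value approaches 90 degrees.
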(event `self.ReceiveBeginPlay`
  (set `self.DefaultScale` (`SceneComponent.RelativeScale3D` (`self.Door_1`))))

(event `self.MoveEvent`
  (if (`self.isOpen`)
    (bind (_direction _newtrack_0) (`Timeline|OpenClose` :!label _label)
      (:`Update`
        (`SceneComponent.K2_SetRelativeRotation` (`self.Door_2`) (`KismetMathLibrary.MakeRotator` 90.0 _newtrack_0 90.0) false false)
        (`SceneComponent.K2_SetRelativeRotation` (`self.Door_1`) (`KismetMathLibrary.MakeRotator` 90.0 _newtrack_0 -90.0) false false)
        (bind _returnvalue (* (`self.DefaultScale`) (/ (- 90.0 _newtrack_0) 90.0)))
        (`SceneComponent.SetRelativeScale3D` (`self.Door_1`) _returnvalue)
        (`SceneComponent.SetRelativeScale3D` (`self.Door_2`) _returnvalue)))
    (else
      (goto _label :!via `Reverse`))))

(fn `UserConstructionScript`
  (`parent.UserConstructionScript`))