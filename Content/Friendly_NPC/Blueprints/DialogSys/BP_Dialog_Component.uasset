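; BP_Dialog_Component runs NPC dialog, using a behavior tree as the dialog flow.
; BeginPlay spawns a dedicated AI_DialogController to run that tree.
; ActivateDialog shows a BP_DialogWidget with UI-only input and mouse cursor, runs DialogTree, and stores the widget in its blackboard.
; The widget's exit event restores game input, stops the tree logic and removes the widget.
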(event `self.ReceiveBeginPlay`
  (bind _returnvalue (`|SpawnActorFromClass` "/Game/Friendly_NPC/Blueprints/DialogSys/AI_DialogController.AI_DialogController_C" (`KismetMathLibrary.MakeTransform` (0.0 0.0 0.0)) "Undefined" "OverrideRootScale" null null))
  (set `self.AIController` _returnvalue))

(event `ActivateDialog`
  (bind _returnvalue (`GameplayStatics.GetPlayerController` 0))
  (bind _aicontroller (`self.AIController`))
  (bind _dialogtree (`self.DialogTree`))
  (bind _returnvalue_2 (`|CreateWidget` "/Game/Friendly_NPC/Blueprints/DialogSys/BP_DialogWidget.BP_DialogWidget_C" _returnvalue))
  (bind _output_get (set `self.DialogWidget` _returnvalue_2))
  (add `/Game/Friendly_NPC/Blueprints/DialogSys/BP_DialogWidget.OnExit` _output_get (delegate `OnExit`))
  (`UserWidget.AddToViewport` _output_get 0)
  (`WidgetBlueprintLibrary.SetInputMode_UIOnlyEx` _returnvalue _output_get)
  (set `PlayerController.bShowMouseCursor` true _returnvalue)
  (`AIController.RunBehaviorTree` _aicontroller _dialogtree)
  (bind _blackboardcomponent (`AIController.UseBlackboard` _aicontroller (`BlackboardAssetProvider.GetBlackboardAsset` _dialogtree)))
  (`BlackboardComponent.SetValueAsObject` _blackboardcomponent "DialogWidget" (`self.DialogWidget`)))

(event `OnExit`
  (bind _returnvalue (`GameplayStatics.GetPlayerController` 0))
  (`WidgetBlueprintLibrary.SetInputMode_GameOnly` _returnvalue)
  (set `PlayerController.bShowMouseCursor` false _returnvalue)
  (`BrainComponent.StopLogic` (`AIController.BrainComponent` (`self.AIController`)) "Dialog Exit")
  (`Widget.RemoveFromParent` (`self.DialogWidget`)))