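; BPC_WithWidget is a component that gives its owner a full-screen GUI widget that can be shown and hidden.
; BeginPlay creates the widget once from WidgetType and caches it for reuse.
; ShowGUI and HideGUI add or remove it from the viewport, tinting or untinting the background through the first player's RobotHUD.
; Both functions do nothing if that HUD is not a RobotHUD.
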(event `self.ReceiveBeginPlay`
  (bind _returnvalue (`|CreateWidget` (`self.WidgetType`)))
  (set `self.Widget` _returnvalue))

(fn `HideGUI`
  (bind _asrobot_hud (cast `/Game/FirstPersonBP/Blueprints/RobotHUD` (`PlayerController.GetHUD` (`GameplayStatics.GetPlayerController` 0))))
  (`/Game/FirstPersonBP/Blueprints/RobotHUD.UntintBackground` _asrobot_hud)
  (`Widget.RemoveFromParent` (`self.Widget`)))

(fn `ShowGUI`
  (bind _asrobot_hud (cast `/Game/FirstPersonBP/Blueprints/RobotHUD` (`PlayerController.GetHUD` (`GameplayStatics.GetPlayerController` 0))))
  (`/Game/FirstPersonBP/Blueprints/RobotHUD.TintBackground` _asrobot_hud)
  (`UserWidget.AddToViewport` (`self.Widget`) 0))