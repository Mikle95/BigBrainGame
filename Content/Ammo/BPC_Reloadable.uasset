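; BPC_Reloadable is a Blueprint component that tracks ammo and handles firing and reloading from the player robot's ammo.
; Fire spends one round and returns whether any was available.
; Reload casts player 0 to PlayerRobot and, if below MaxAmmo, waits briefly, requests the shortfall as a negative ChangeAmmo delta, then subtracts the returned change to refill Ammo.
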(event `Reload`
  (bind _ammo (`self.Ammo`))
  (bind _asplayer_robot (cast `/Game/FirstPersonBP/Blueprints/PlayerRobot` (`GameplayStatics.GetPlayerCharacter` 0)))
  (if (> (`self.MaxAmmo`) (`self.Ammo`))
    (`KismetSystemLibrary.Delay` 0.1)
    (bind _change (`/Game/FirstPersonBP/Blueprints/PlayerRobot.ChangeAmmo` _asplayer_robot (- _ammo (`self.MaxAmmo`))))
    (set `self.Ammo` (- _ammo _change))))

(fn `Fire`
  (returns (Success :type Boolean))
  (if (> (`self.Ammo`) 0)
    (`/Engine/EditorBlueprintResources/StandardMacros.DecrementInt` (`self.Ammo`)
      (:`  `
        (return true)))
    (else
      (return false))))